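; ExplosiveCrystal is a short-lived weapon actor that grows into the world and shrinks away; no explosion or damage logic appears here.
; On spawn it picks a random lifespan, applies a random yaw with slight tilt, plays an opening sound and scales up through the Grow timeline.
; Tick counts down the lifespan, then reverses Grow once; the reversed finish plays a closing sound and destroys the actor.
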(event EventBeginPlay
  (bind _returnvalue (Math|Random|RandomRotator false))
  (Variables|Default|Setlifespan (Math|Random|RandomFloatinRange 8.0 1e+01))
  (Transformation|SetActorRotation (Math|Rotator|MakeRotator 0.0 (* (.pitch _returnvalue) 0.05) (.yaw _returnvalue)) true)
  (Audio|PlaySoundatLocation "/Engine/VREditor/Sounds/VR_open_Cue.VR_open_Cue" (Transformation|GetActorLocation) "0, 0, 0" 0.5 1.0 0.0 0 0 0)
  (bind (_direction _scale) (Timeline|Grow Play)
    (:Update
      (Transformation|SetActorScale3D (Math|Vector|MakeVector _scale _scale _scale)))
    (:Finished
      (switch Utilities|FlowControl|Switch|SwitchonETimelineDirection _direction
        (:Backward
          (Audio|PlaySoundatLocation "/Engine/VREditor/Sounds/VR_close_Cue.VR_close_Cue" (Transformation|GetActorLocation) "0, 0, 0" 0.5 1.0 0.0 0 0 0)
          (Actor|DestroyActor))))))

(event EventTick
  (params (DeltaSeconds :type Float%20%28single-precision%29))
  (bind _output_get (Variables|Default|Setlifespan (- (Variables|Default|Getlifespan) DeltaSeconds)))
  (if (<= _output_get 0.0)
    (if (not (Variables|Default|GetisDead))
      (Variables|Default|SetisDead true)
      (bind (_direction _scale) (Timeline|Grow ReverseFromEnd)
        (:Update
          (Transformation|SetActorScale3D (Math|Vector|MakeVector _scale _scale _scale)))
        (:Finished
          (switch Utilities|FlowControl|Switch|SwitchonETimelineDirection _direction
            (:Backward
              (Audio|PlaySoundatLocation "/Engine/VREditor/Sounds/VR_close_Cue.VR_close_Cue" (Transformation|GetActorLocation) "0, 0, 0" 0.5 1.0 0.0 0 0 0)
              (Actor|DestroyActor))))))))

(fn ConstructionScript)