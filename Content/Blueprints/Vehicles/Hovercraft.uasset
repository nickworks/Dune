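; Hovercraft Blueprint that floats on four physics thrusters attached to a box body sized by VehicleSize in the construction script.
; Each tick, every thruster sphere-traces along its forward vector and sets its strength from a falloff curve of normalized hit distance times HoverStrength.
; A corrective torque from the cross product of the box's up vector and world up keeps the craft upright.
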(event EventBeginPlay)

(event Collision|EventActorBeginOverlap
  (params (OtherActor :type Actor%20Object%20Reference)))

(event EventTick
  (params (DeltaSeconds :type Float%20%28single-precision%29))
  (CallFunction|Hover))

(fn ConstructionScript
  (bind _vehicle_size (Variables|Default|GetVehicle%20Size))
  (Components|Box|SetBoxExtent (Variables|Default|GetBox) (/ _vehicle_size 2.0) true)
  (Transformation|SetRelativeScale3D (Variables|Default|GetMesh%20body) (/ _vehicle_size 1e+02))
  (Variables|Default|SetThrusters (Utilities|Array|MakeArray (Variables|Default|GetPhysicsThruster2) (Variables|Default|GetPhysicsThruster3) (Variables|Default|GetPhysicsThruster) (Variables|Default|GetPhysicsThruster1))))

(fn Hover
  (bind _box (Variables|Default|GetBox))
  (for _array_element (Variables|Default|GetThrusters)
    (CallFunction|ModulateStrength _array_element))
  (Class|PrimitiveComponent|AddTorqueinDegrees _box (* (Math|Vector|CrossProduct (Math|Vector|GetUpVector _box) (Math|Vector|VectorUp)) (Variables|Default|GetUpright%20Torque)) "None" false))

(fn ModulateStrength
  (params (Thruster :type Physics%20Thruster%20Component%20Object%20Reference))
  (bind _returnvalue (Transformation|GetWorldLocation Thruster))
  (bind (_outhit _returnvalue_2) (Collision|SphereTraceByChannel _returnvalue (+ _returnvalue (* (Math|Vector|GetForwardVector Thruster) (Variables|Default|GetHoverDetectDistance))) 5.0 "TraceTypeQuery1" false 0 "ForOneFrame"))
  (Variables|/Script/Engine.PhysicsThrusterComponent|SetThrustStrength Thruster (* (Variables|Default|GetHoverStrength) (Math|Curves|GetFloatValue (Variables|Default|GetHoverStrengthFalloff) (select _returnvalue_2 (/ (.Distance (Collision|BreakHitResult _outhit)) (Variables|Default|GetHoverDetectDistance)) 1.0)))))