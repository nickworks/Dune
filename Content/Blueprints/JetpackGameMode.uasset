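; Game mode for a jetpack game that tracks the current checkpoint and respawns the player.
; SetCheckpoint stores the given checkpoint as CurrentCheckpoint.
; Respawn uses the checkpoint passed in rather than the stored one: it destroys player 0's pawn, spawns a new JetpackCharacter at that RespawnPoint's location and rotation, and possesses it.
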(fn ConstructionScript)

(fn Respawn
  (params (At :type Checkpoint%20Object%20Reference))
  (bind _returnvalue (Game|GetPlayerController 0))
  (bind _respawn_point (Variables|/Game/Blueprints/Checkpoint.Checkpoint_C|GetRespawn%20point At))
  (bind _returnvalue_2 (Transformation|GetWorldTransform _respawn_point))
  (bind _returnvalue_3 (Pawn|GetControlledPawn _returnvalue))
  (Utilities|IsValid _returnvalue_3
    (:Is%20Valid
      (Actor|DestroyActor _returnvalue_3))
    (:Is%20Not%20Valid
      _))
  (bind _returnvalue_4 (Game|SpawnActorfromClass "/Game/Blueprints/PlayerCharacter/JetpackCharacter.JetpackCharacter_C" (Math|Transform|MakeTransform (.location _returnvalue_2) (.rotation _returnvalue_2) "1,1,1") "Undefined" 0 0))
  (Pawn|Possess (Game|GetPlayerController 0) _returnvalue_4))

(fn SetCheckpoint
  (params (Checkpoint :type Checkpoint%20Object%20Reference))
  (Variables|Default|SetCurrentCheckpoint Checkpoint))